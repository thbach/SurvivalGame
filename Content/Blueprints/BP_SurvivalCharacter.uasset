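; BP_SurvivalCharacter is a survival character Blueprint assembled from modular gear meshes with an attached camera.
; Its construction script makes the backpack, helmet, chest, legs, feet, vest and hands meshes follow the main Mesh's animation through master pose.
; It also attaches the camera to the Mesh's CameraSocket, keeping relative location, rotation and scale.
; BeginPlay only prints whether that socket exists, as a debug check.
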(event `self.ReceiveBeginPlay`
  (`KismetSystemLibrary.PrintString` (`KismetStringLibrary.Conv_BoolToString` (`SceneComponent.DoesSocketExist` (`self.Mesh`) "CameraSocket"))))

(fn `UserConstructionScript`
  (bind _mesh (`self.Mesh`))
  (`SkinnedMeshComponent.SetLeaderPoseComponent` (`self.BackpackMesh`) _mesh false)
  (`SkinnedMeshComponent.SetLeaderPoseComponent` (`self.HelmetMesh`) _mesh false)
  (`SkinnedMeshComponent.SetLeaderPoseComponent` (`self.ChestMesh`) _mesh false)
  (`SkinnedMeshComponent.SetLeaderPoseComponent` (`self.LegsMesh`) _mesh false)
  (`SkinnedMeshComponent.SetLeaderPoseComponent` (`self.FeetMesh`) _mesh false)
  (`SkinnedMeshComponent.SetLeaderPoseComponent` (`self.VestMesh`) _mesh false)
  (`SkinnedMeshComponent.SetLeaderPoseComponent` (`self.HandsMesh`) _mesh false)
  (`SceneComponent.K2_AttachToComponent` (`self.CameraComponent`) _mesh "CameraSocket" "KeepRelative" "KeepRelative" "KeepRelative" true))